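; Pannel is a Blueprint that switches a scene capture camera between four feeds, apparently for an in-world camera panel.
; Each CameraFeed event moves and rotates the Scene capture component to its own stored location and rotation, then plays an audio component.
; An unconnected snippet would show the mouse cursor and set Game-and-UI input focused on the widget, but never runs.
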(event EventCameraFeed01
  (bind _scene_ (Variables|Default|Getscene%20))
  (bind _capturecomponent2d (Variables|/Script/Engine.SceneCapture2D|GetCaptureComponent2D _scene_))
  (Utilities|FlowControl|Sequence
    (:then_0
      (Transformation|SetWorldLocation _capturecomponent2d (Variables|Default|GetLocation01) false false))
    (:then_1
      (Transformation|SetWorldRotation _capturecomponent2d (Variables|Default|GetRotation01) false false))
    (:then_2
      (Audio|Components|Audio|Play (Variables|Default|GetAudio) 0.0))))

(event EventCameraFeed02
  (bind _scene_ (Variables|Default|Getscene%20))
  (bind _capturecomponent2d (Variables|/Script/Engine.SceneCapture2D|GetCaptureComponent2D _scene_))
  (Utilities|FlowControl|Sequence
    (:then_0
      (Transformation|SetWorldLocation _capturecomponent2d (Variables|Default|GetLocation02) false false))
    (:then_1
      (Transformation|SetWorldRotation _capturecomponent2d (Variables|Default|GetRotation02) false false))
    (:then_2
      (Audio|Components|Audio|Play (Variables|Default|GetAudio) 0.0))))

(event EventCameraFeed03
  (bind _scene_ (Variables|Default|Getscene%20))
  (bind _capturecomponent2d (Variables|/Script/Engine.SceneCapture2D|GetCaptureComponent2D _scene_))
  (Utilities|FlowControl|Sequence
    (:then_0
      (Transformation|SetWorldLocation _capturecomponent2d (Variables|Default|GetLocation03) false false))
    (:then_1
      (Transformation|SetWorldRotation _capturecomponent2d (Variables|Default|GetRotation03) false false))
    (:then_2
      (Audio|Components|Audio|Play (Variables|Default|GetAudio) 0.0))))

(event EventCameraFeed04
  (bind _scene_ (Variables|Default|Getscene%20))
  (bind _capturecomponent2d (Variables|/Script/Engine.SceneCapture2D|GetCaptureComponent2D _scene_))
  (Utilities|FlowControl|Sequence
    (:then_0
      (Transformation|SetWorldLocation _capturecomponent2d (Variables|Default|GetLocation04) false false))
    (:then_1
      (Transformation|SetWorldRotation _capturecomponent2d (Variables|Default|GetRotation04) false false))
    (:then_2
      (Audio|Components|Audio|Play (Variables|Default|GetAudio) 0.0))))

(fn ConstructionScript)

(fn NewFunction0)