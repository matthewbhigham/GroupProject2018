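; A keypad-locked door Blueprint that swings according to the player's facing direction and closes when the player leaves its box.
; KeyPad01 opens a Gate that unlocks Interact and immediately triggers a looping MultiGate that alternates opening and closing.
; The sign of the player's world forward X picks one of two timelines, whose summed outputs drive door yaw.
; Closing reverses the chosen timeline, and exiting the box also resets the MultiGate.
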(event OnComponentEndOverlap(Box)
  (params (OverlappedComponent :type Primitive%20Component%20Object%20Reference) (OtherActor :type Actor%20Object%20Reference) (OtherComp :type Primitive%20Component%20Object%20Reference) (OtherBodyIndex :type Integer))
  (bind _returnvalue (Game|GetPlayerCharacter 0))
  ;[1 1 1] Door Open and Close Depending On player Pirection.
  (if (== OtherActor _returnvalue)
    (Utilities|FlowControl|Sequence
      (:then_0
        (Utilities|FlowControl|MultiGate false true -1) ; enters at Reset
      )
      (:then_1
        (if (Variables|Default|GetSetDirection)
          (bind _dooropening (Timeline|Timeline_0 Reverse)
            (:Update
              _))
          (else
            (bind _dooropening_2 (Timeline|Timeline_1 Reverse)
              (:Update
                _))))
        (Transformation|SetRelativeRotation (Variables|Default|GetSM_Door) (Math|Rotator|MakeRotator 0.0 0.0 (+ _dooropening (.Pitch (Math|Rotator|BreakRotator (Variables|Default|GetDoorStartRotation))) _dooropening_2)) false false)))))

(event EventKeyPad01
  ;[1 1 1] Door Open and Close Depending On player Pirection.
  (Utilities|FlowControl|Sequence
    (:then_0
      (Utilities|FlowControl|Gate true) ; enters at Open
    )
    (:then_1
      (Utilities|FlowControl|MultiGate false true -1
        (:Out%200
          (Math|Float|CompareFloat (.X (Math|Vector|BreakVector (Transformation|GetActorForwardVector (Game|GetPlayerCharacter 0)))) 0.0
            (:>
              (Variables|Default|SetSetDirection true)
              (bind _dooropening (Timeline|Timeline_0 Play)
                (:Update
                  (Transformation|SetRelativeRotation (Variables|Default|GetSM_Door) (Math|Rotator|MakeRotator 0.0 0.0 (+ _dooropening (.Pitch (Math|Rotator|BreakRotator (Variables|Default|GetDoorStartRotation))) (stale _dooropening_2))) false false :!label _label))))
            (:<
              (Variables|Default|SetSetDirection false)
              (bind _dooropening_2 (Timeline|Timeline_1 Play)
                (:Update
                  (goto _label))))))
        (:Out%201
          (if (Variables|Default|GetSetDirection)
            (Timeline|Timeline_0 Reverse)
            (else
              (Timeline|Timeline_1 Reverse))))))))

(event EventInteract
  ;[1 1 1] Door Open and Close Depending On player Pirection.
  (Utilities|FlowControl|Gate true
    (:Exit
      (Utilities|FlowControl|MultiGate false true -1
        (:Out%200
          (Math|Float|CompareFloat (.X (Math|Vector|BreakVector (Transformation|GetActorForwardVector (Game|GetPlayerCharacter 0)))) 0.0
            (:>
              (Variables|Default|SetSetDirection true)
              (bind _dooropening (Timeline|Timeline_0 Play)
                (:Update
                  (Transformation|SetRelativeRotation (Variables|Default|GetSM_Door) (Math|Rotator|MakeRotator 0.0 0.0 (+ _dooropening (.Pitch (Math|Rotator|BreakRotator (Variables|Default|GetDoorStartRotation))) (stale _dooropening_2))) false false :!label _label))))
            (:<
              (Variables|Default|SetSetDirection false)
              (bind _dooropening_2 (Timeline|Timeline_1 Play)
                (:Update
                  (goto _label))))))
        (:Out%201
          (if (Variables|Default|GetSetDirection)
            (Timeline|Timeline_0 Reverse)
            (else
              (Timeline|Timeline_1 Reverse))))))))

(fn ConstructionScript)