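; VentDoor_01 is an interactable vent door that slides its panel open and closed.
; Each Interact call alternates through a looping MultiGate between playing and reversing a Timeline.
; The Timeline's PannelMovement track lerps the SMDoor mesh's relative transform between start and end locations.
; When the player character leaves the Box trigger, the MultiGate resets and the Timeline reverses to close the door.
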(event OnComponentEndOverlap(Box)
  (params (OverlappedComponent :type Primitive%20Component%20Object%20Reference) (OtherActor :type Actor%20Object%20Reference) (OtherComp :type Primitive%20Component%20Object%20Reference) (OtherBodyIndex :type Integer))
  ;[1 1 1] Door Open and Close Depending On player Pirection.
  (if (== OtherActor (Game|GetPlayerCharacter 0))
    (Utilities|FlowControl|Sequence
      (:then_0
        (Utilities|FlowControl|MultiGate false true -1) ; enters at Reset
      )
      (:then_1
        (bind _pannelmovement (Timeline|Timeline_0 Reverse)
          (:Update
            (Transformation|SetRelativeTransform (Variables|Default|GetSM_Door) (Math|Conversions|ToTransform(Vector) (Math|Vector|Lerp(Vector) (Variables|Default|GetDoorStartLocation) (Variables|Default|GetDoorEndLocation) _pannelmovement)) false false)))))))

(event EventInteract
  ;[1 1 1] Door Open and Close Depending On player Pirection.
  (Utilities|FlowControl|MultiGate false true -1
    (:Out%200
      (bind _pannelmovement (Timeline|Timeline_0 Play)
        (:Update
          (Transformation|SetRelativeTransform (Variables|Default|GetSM_Door) (Math|Conversions|ToTransform(Vector) (Math|Vector|Lerp(Vector) (Variables|Default|GetDoorStartLocation) (Variables|Default|GetDoorEndLocation) _pannelmovement)) false false))))
    (:Out%201
      (Timeline|Timeline_0 Reverse))))

(fn ConstructionScript)